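; Loop manager that layers kick, snare, hi-hat and piano MetaSound loops as BP_Player enters each instrument's collision.
; BeginPlay starts a 4/4 Quartz clock and plays all four MetaSounds.
; Each overlap subscribes to the clock's Bar boundary, whose callback sends that MetaSound's "Start" trigger, keeping layers musically quantized.
; Per-instrument events also forward named toggle triggers to the MetaSounds, with debug prints for toggles and bar:beat position.
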(event OnComponentBeginOverlap(KickCollision)
  (params (OverlappedComponent :type Primitive%20Component%20Object%20Reference) (OtherActor :type Actor%20Object%20Reference) (OtherComp :type Primitive%20Component%20Object%20Reference) (OtherBodyIndex :type Integer) (bFromSweep :type Boolean) (SweepResult :type Hit%20Result%20Structure%20%28by%20ref%29))
  (if (== (Utilities|GetClass OtherActor) "/Game/Blueprints/Core/BP_Player.BP_Player_C")
    (Class|QuartzClockHandle|SubscribetoQuantizationEvent (Variables|Default|GetQuartzClock) "Bar" (delegate Custom|StartKick))))

(event OnComponentBeginOverlap(SnareCollision)
  (params (OverlappedComponent :type Primitive%20Component%20Object%20Reference) (OtherActor :type Actor%20Object%20Reference) (OtherComp :type Primitive%20Component%20Object%20Reference) (OtherBodyIndex :type Integer) (bFromSweep :type Boolean) (SweepResult :type Hit%20Result%20Structure%20%28by%20ref%29))
  (if (== (Utilities|GetClass OtherActor) "/Game/Blueprints/Core/BP_Player.BP_Player_C")
    (Class|QuartzClockHandle|SubscribetoQuantizationEvent (Variables|Default|GetQuartzClock) "Bar" (delegate Custom|CustomEvent))))

(event OnComponentBeginOverlap(HihatCollision)
  (params (OverlappedComponent :type Primitive%20Component%20Object%20Reference) (OtherActor :type Actor%20Object%20Reference) (OtherComp :type Primitive%20Component%20Object%20Reference) (OtherBodyIndex :type Integer) (bFromSweep :type Boolean) (SweepResult :type Hit%20Result%20Structure%20%28by%20ref%29))
  (if (== (Utilities|GetClass OtherActor) "/Game/Blueprints/Core/BP_Player.BP_Player_C")
    (Class|QuartzClockHandle|SubscribetoQuantizationEvent (Variables|Default|GetQuartzClock) "Bar" (delegate Custom|CustomEvent_1))))

(event OnComponentBeginOverlap(PianoCollision)
  (params (OverlappedComponent :type Primitive%20Component%20Object%20Reference) (OtherActor :type Actor%20Object%20Reference) (OtherComp :type Primitive%20Component%20Object%20Reference) (OtherBodyIndex :type Integer) (bFromSweep :type Boolean) (SweepResult :type Hit%20Result%20Structure%20%28by%20ref%29))
  (if (== (Utilities|GetClass OtherActor) "/Game/Blueprints/Core/BP_Player.BP_Player_C")
    (Class|QuartzClockHandle|SubscribetoQuantizationEvent (Variables|Default|GetQuartzClock) "Bar" (delegate Custom|StartPiano))))

(event Custom|BarEvents
  (params (ClockName :type Name) (QuantizationType :type EQuartzCommandQuantization%20Enum :default "Bar") (NumBars :type Integer) (Beat :type Integer) (BeatFraction :type Float%20%28single-precision%29))
  (Development|PrintString (Utilities|String|Append (Utilities|String|ToString(Integer) NumBars) ":" (Utilities|String|ToString(Integer) Beat))))

(event Custom|CustomEvent_1
  (params (ClockName :type Name) (QuantizationType :type EQuartzCommandQuantization%20Enum :default "Bar") (NumBars :type Integer) (Beat :type Integer) (BeatFraction :type Float%20%28single-precision%29))
  (Class|AudioParameterControllerInterface|SetTriggerParameter (Variables|Default|GetHiHatMetaSound) "Start"))

(event Custom|StartKick
  (params (ClockName :type Name) (QuantizationType :type EQuartzCommandQuantization%20Enum :default "Bar") (NumBars :type Integer) (Beat :type Integer) (BeatFraction :type Float%20%28single-precision%29))
  (Class|AudioParameterControllerInterface|SetTriggerParameter (Variables|Default|GetKickMetaSound) "Start"))

(event Custom|StartPiano
  (params (ClockName :type Name) (QuantizationType :type EQuartzCommandQuantization%20Enum :default "Bar") (NumBars :type Integer) (Beat :type Integer) (BeatFraction :type Float%20%28single-precision%29))
  (Class|AudioParameterControllerInterface|SetTriggerParameter (Variables|Default|GetPianoMetaSound) "Start"))

(event Custom|CustomEvent
  (params (ClockName :type Name) (QuantizationType :type EQuartzCommandQuantization%20Enum :default "Bar") (NumBars :type Integer) (Beat :type Integer) (BeatFraction :type Float%20%28single-precision%29))
  (Class|AudioParameterControllerInterface|SetTriggerParameter (Variables|Default|GetSnareMetaSound) "Start"))

(event EventBeginPlay
  (bind _returnvalue (Class|QuartzSubsystem|CreateNewClock (WorldSubsystems|GetQuartzSubsystem) "MainClock" (Utilities|Struct|MakeQuartzClockSettings (Utilities|Struct|MakeQuartzTimeSignature 4 "QuarterNote") false) false))
  (bind _clockhandle (Class|QuartzClockHandle|SetBeatsPerMinute :self _returnvalue :BeatsPerMinute (Variables|Default|GetBeats%20Per%20Minute)))
  (bind _clockhandle_2 (Class|QuartzClockHandle|SubscribetoQuantizationEvent _clockhandle "Beat" (delegate Custom|BarEvents)))
  (bind _output_get (Variables|Default|SetQuartzClock _clockhandle_2))
  (Class|QuartzClockHandle|StartClock _output_get)
  (bind _returnvalue_2 (Audio|CreateSound2D "/Game/Sounds/MS_KickLoop.MS_KickLoop" 1.0 1.0 0.0 0))
  (bind _output_get_2 (Variables|Default|SetKickMetaSound _returnvalue_2))
  (Audio|Components|Audio|Play _output_get_2 0.0)
  (bind _returnvalue_3 (Audio|CreateSound2D "/Game/Sounds/MS_SnareLoop.MS_SnareLoop" 1.0 1.0 0.0 0))
  (bind _output_get_3 (Variables|Default|SetSnareMetaSound _returnvalue_3))
  (Audio|Components|Audio|Play _output_get_3 0.0)
  (bind _returnvalue_4 (Audio|CreateSound2D "/Game/Sounds/MS_HiHatLoop.MS_HiHatLoop" 1.0 1.0 0.0 0))
  (bind _output_get_4 (Variables|Default|SetHiHatMetaSound _returnvalue_4))
  (Audio|Components|Audio|Play _output_get_4 0.0)
  (bind _returnvalue_5 (Audio|CreateSound2D "/Game/Sounds/MS_PianoLoop.MS_PianoLoop" 1.0 1.0 0.0 0))
  (bind _output_get_5 (Variables|Default|SetPianoMetaSound _returnvalue_5))
  (Audio|Components|Audio|Play _output_get_5 0.0))

(event EventSnareTrigger
  (params (ToggleName :type Name :default "None"))
  (Class|AudioParameterControllerInterface|SetTriggerParameter (Variables|Default|GetSnareMetaSound) ToggleName)
  (Development|PrintString (Utilities|String|ToString(Name) ToggleName)))

(event EventPianoTrigger
  (params (ToggleName :type Name :default "None") (Semitone :type Float%20%28double-precision%29))
  (Class|AudioParameterControllerInterface|SetTriggerParameter (Variables|Default|GetPianoMetaSound) ToggleName)
  (Development|PrintString (Utilities|String|ToString(Name) ToggleName)))

(event EventHiHatTrigger
  (params (ToggleName :type Name :default "None"))
  (Class|AudioParameterControllerInterface|SetTriggerParameter (Variables|Default|GetHiHatMetaSound) ToggleName)
  (Development|PrintString (Utilities|String|ToString(Name) ToggleName)))

(event EventKickTrigger
  (params (ToggleName :type Name :default "None"))
  (Class|AudioParameterControllerInterface|SetTriggerParameter (Variables|Default|GetKickMetaSound) ToggleName)
  (Development|PrintString (Utilities|String|ToString(Name) ToggleName)))

(fn ConstructionScript)