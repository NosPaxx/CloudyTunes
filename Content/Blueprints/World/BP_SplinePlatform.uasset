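; Spline platform that moves a scene component along a spline, with options for autostart, looping and reversing.
; A timeline maps its value to distance along the spline, sweeping location and optionally applying the spline's roll and yaw.
; The React event starts looping or reversing platforms once when not autostarted, and toggles direction on one-way platforms.
; When the timeline finishes, Reverse flip-flops playback direction if reversing is enabled.
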(event EventBeginPlay
  (Components|Timeline|SetPlayRate (Variables|Default|GetMoveTimeline) (|(1/{CB70A40D-42FC-8A61-D851-55A0C542E628})))
  (Components|Timeline|SetLooping (Variables|Default|GetMoveTimeline) (Variables|Default|GetCanLoop))
  (Variables|Default|GetAutostart
    (:then
      (Audio|Components|Audio|Play (Variables|Default|GetMoveTimeline)))
    (:else)))

(event EventReact
  (Utilities|FlowControl|Sequence
    (:then_0
      (if (Math|Boolean|ANDBoolean (Variables|Default|GetAutostart) (not (Variables|Default|GetCanLoop)) (not (Variables|Default|GetCanReverse)))
        (Utilities|FlowControl|FlipFlop
          (:A
            (Utilities|String|Reverse (Variables|Default|GetMoveTimeline)))
          (:B
            (Audio|Components|Audio|Play (Variables|Default|GetMoveTimeline))))))
    (:then_1
      (if (and (not (Variables|Default|GetAutostart)) (or (Variables|Default|GetCanLoop) (Variables|Default|GetCanReverse)))
        (Utilities|FlowControl|DoOnce false
          (:Completed
            (Audio|Components|Audio|Play (Variables|Default|GetMoveTimeline))))))
    (:then_2
      (if (Math|Boolean|ANDBoolean (not (Variables|Default|GetAutostart)) (not (Variables|Default|GetCanLoop)) (not (Variables|Default|GetCanReverse)))
        (Utilities|FlowControl|FlipFlop
          (:A
            (Audio|Components|Audio|Play (Variables|Default|GetMoveTimeline)))
          (:B
            (Utilities|String|Reverse (Variables|Default|GetMoveTimeline))))))))

(fn ConstructionScript)