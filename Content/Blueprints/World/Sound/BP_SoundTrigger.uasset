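; BP_SoundTrigger is a trigger box that signals the loop manager to change an instrument part when the player overlaps it.
; On overlap it finds all BP_LoopManager actors and, based on its Instrument enum, sends a kick, snare, hi-hat or piano message carrying its toggle variable.
; The piano branch passes a fixed zero semitone, leaving the Semitone variable unused, and prints debug strings.
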(event OnComponentBeginOverlap(Box)
  (params (OverlappedComponent :type Primitive%20Component%20Object%20Reference) (OtherActor :type Actor%20Object%20Reference) (OtherComp :type Primitive%20Component%20Object%20Reference) (OtherBodyIndex :type Integer) (bFromSweep :type Boolean) (SweepResult :type Hit%20Result%20Structure%20%28by%20ref%29))
  (if (== (Utilities|GetClass OtherActor) "/Game/Blueprints/Core/BP_Player.BP_Player_C")
    (bind _outactors (Actor|GetAllActorsOfClass "/Game/Blueprints/World/BP_LoopManager.BP_LoopManager_C"))
    (if (Utilities|Enum|Equal(Enum) (Variables|Default|GetInstrument) "NewEnumerator0")
      (Class|BPIAudioTrigger|KickTrigger(Message) _outactors (Variables|Default|GetToogleVariable))
      (elif (Utilities|Enum|Equal(Enum) (Variables|Default|GetInstrument) "NewEnumerator1")
        (Class|BPIAudioTrigger|SnareTrigger(Message) _outactors (Variables|Default|GetToogleVariable))
        (elif (Utilities|Enum|Equal(Enum) (Variables|Default|GetInstrument) "NewEnumerator2")
          (Class|BPIAudioTrigger|HiHatTrigger(Message) _outactors (Variables|Default|GetToogleVariable))
          (elif (Utilities|Enum|Equal(Enum) (Variables|Default|GetInstrument) "NewEnumerator3")
            (Development|PrintString "Hello")
            (Class|BPIAudioTrigger|PianoTrigger(Message) _outactors (Variables|Default|GetToogleVariable) 0.0)
            (Development|PrintString "triggged")))))))

(fn ConstructionScript)