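; BP_C_PressurePlate is a pressure plate actor that responds when the player steps into its trigger box.
; The Box overlap checks for an exact BP_Player class match, then uses MoveComponentTo to slide SMPlate along relative Y with eased motion over two seconds.
; No end-overlap or reset logic returns the plate to its start position, and it signals no other actor.
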(event OnComponentBeginOverlap(Box)
  (params (OverlappedComponent :type Primitive%20Component%20Object%20Reference) (OtherActor :type Actor%20Object%20Reference) (OtherComp :type Primitive%20Component%20Object%20Reference) (OtherBodyIndex :type Integer) (bFromSweep :type Boolean) (SweepResult :type Hit%20Result%20Structure%20%28by%20ref%29))
  (if (== (Utilities|GetClass OtherActor) "/Game/Blueprints/Core/BP_Player.BP_Player_C")
    (Components|MoveComponentTo (Variables|Default|GetSM_Plate) "0.000000,200.000000,0.000000" "0, 0, 0" true true 2.0 false)))

(event EventBeginPlay
  (|CallParentFunction))

(event Collision|EventActorBeginOverlap
  (params (OtherActor :type Actor%20Object%20Reference))
  (|CallParentFunction OtherActor) ; This node is disabled and will not be called.\nDrag off pins to build functionality.
)

(event EventTick
  (params (DeltaSeconds :type Float%20%28single-precision%29))
  (|CallParentFunction DeltaSeconds) ; This node is disabled and will not be called.\nDrag off pins to build functionality.
)

(fn ConstructionScript
  (|CallParentFunction))