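; BP_Interactable is a world actor that players can interact with to trigger reactions in other actors.
; Its sphere overlap registers or unregisters it with BPI_Player actors and toggles a highlight overlay material and billboard prompt.
; Interact sends ReactMessage to ActorsToReact, with optional one-time use and optional self-destruction after removing itself from the sender's interactables.
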(event OnComponentBeginOverlap(Sphere)
  (params (OverlappedComponent :type Primitive%20Component%20Object%20Reference) (OtherActor :type Actor%20Object%20Reference) (OtherComp :type Primitive%20Component%20Object%20Reference) (OtherBodyIndex :type Integer) (bFromSweep :type Boolean) (SweepResult :type Hit%20Result%20Structure%20%28by%20ref%29))
  (if (Utilities|DoesObjectImplementInterface OtherActor "/Game/Blueprints/Interfaces/BPI_Player.BPI_Player_C")
    (Class|BPIPlayer|UpdateInteractables(Message) OtherActor self true)
    (Variables|Default|GetInteractOnce
      (:then
        (Variables|Default|GetFirstInteract
          (:then
            _)
          (:else)))
      (:else
        _))
    (Rendering|Material|SetOverlayMaterial (Variables|Default|GetMesh) "/Game/Materials/MI_InteractableOverlay.MI_InteractableOverlay" :!class /Script/Engine.MeshComponent)
    (Development|SetHiddeninGame (Variables|Default|GetBillboard) false false)))

(event OnComponentEndOverlap(Sphere)
  (params (OverlappedComponent :type Primitive%20Component%20Object%20Reference) (OtherActor :type Actor%20Object%20Reference) (OtherComp :type Primitive%20Component%20Object%20Reference) (OtherBodyIndex :type Integer))
  (if (Utilities|DoesObjectImplementInterface OtherActor "/Game/Blueprints/Interfaces/BPI_Player.BPI_Player_C")
    (Class|BPIPlayer|UpdateInteractables(Message) OtherActor self false)
    (Rendering|Material|SetOverlayMaterial (Variables|Default|GetMesh) 0 :!class /Script/Engine.MeshComponent)
    (Development|SetHiddeninGame (Variables|Default|GetBillboard) true false)))

(event EventInteract
  (params (Sender :type Actor%20Object%20Reference))
  (Variables|Default|GetInteractOnce
    (:then
      (Variables|Default|GetFirstInteract
        (:then
          (Variables|Default|SetFirstInteract false)
          (Rendering|Material|SetOverlayMaterial (Variables|Default|GetMesh) "/Game/Materials/M_overlay.M_overlay" :!class /Script/Engine.MeshComponent))
        (:else)))
    (:else
      _))
  (Class|BPIReact|React(Message) (Variables|Default|GetActorsToReact))
  (Variables|Default|GetDestroyOnInteract
    (:then
      (Class|BPIPlayer|UpdateInteractables(Message) Sender self false)
      (Actor|DestroyActor))
    (:else)))

(fn ConstructionScript)