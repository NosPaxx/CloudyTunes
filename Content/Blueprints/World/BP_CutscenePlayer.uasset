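; World actor that plays an assigned level sequence cutscene when its React event fires, gated by PlayOnce and a DoOnce.
; For cutscenes flagged HasCamera, it increments the player's CanMove counter and pushes a cutscene widget onto the HUD's main widget stack.
; The sequence player's OnFinished callback reverses both, decrementing the counter and removing the widget.
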(event Custom|OnFinished
  (Variables|Default|GetHasCamera
    (:then
      (bind _as_bp_player (Variables|Default|GetAs%20BP%20Player)
        (:then
          (Math|Integer|DecrementInt (Variables|/Game/Blueprints/Core/BP_Player.BP_Player_C|GetCanMove _as_bp_player)
            (:%20%20
              (Class|CommonActivatableWidgetContainerBase|RemoveWidget (CallFunction|ReturnMainStack (Game|GetPlayerController 0)) (Variables|Default|GetWidget)))))
        (:else)))
    (:else)))

(event EventBeginPlay)

(event Collision|EventActorBeginOverlap
  (params (OtherActor :type Actor%20Object%20Reference)))

(event EventTick
  (params (DeltaSeconds :type Float%20%28single-precision%29)))

(event EventReact
  (bind _cutscenetoplay (Variables|Default|GetCutSceneToPlay)
    (:then
      (Variables|Default|GetPlayOnce
        (:then
          (Utilities|FlowControl|DoOnce false
            (:Completed
              (Utilities|FlowControl|Sequence
                (:then_0
                  (Variables|Default|GetAs%20BP%20Player
                    (:then)
                    (:else
                      (bind _asbp_player (Utilities|Casting|CastToBP_Player (Game|GetPlayerCharacter 0)))
                      (Variables|Default|SetAs%20BP%20Player _asbp_player))))
                (:then_1
                  (EventDispatchers|BindEventtoOnFinished (Variables|/Script/LevelSequence.LevelSequenceActor|GetSequencePlayer (Variables|Default|GetCutSceneToPlay)) (EventDispatchers|CreateEvent :!event Custom|OnFinished)))
                (:then_2
                  (Variables|Default|GetHasCamera
                    (:then
                      (Math|Integer|IncrementInt (Variables|/Game/Blueprints/Core/BP_Player.BP_Player_C|GetCanMove (Variables|Default|GetAs%20BP%20Player))
                        (:%20%20
                          (bind _mainwidget (Class|BPIHUD|ReturnMainWidget(Message) (HUD|GetHUD (Game|GetPlayerController 0))))
                          (bind _returnvalue (Class|CommonActivatableWidgetContainerBase|AddWidget (Variables|/Game/Blueprints/UI/CUW_Main.CUW_Main_C|GetMainStack _mainwidget) "/Game/Blueprints/UI/CAW_CutScene.CAW_CutScene_C"))
                          (Variables|Default|SetWidget _returnvalue))))
                    (:else)))
                (:then_3
                  (Sequencer|Player|Play (Variables|/Script/LevelSequence.LevelSequenceActor|GetSequencePlayer _cutscenetoplay) :!class /Script/MovieScene.MovieSceneSequencePlayer))))))
        (:else)))
    (:else)))

(fn ConstructionScript)