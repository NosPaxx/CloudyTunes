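; BP_Collectable is a world pickup that adds its Value to a total through the game mode when the player collects it.
; On BeginPlay the CoinRotate timeline spins and bobs its Scene component.
; A sphere overlap with BP_Player fires once, starting the Collect timeline, which lerps the actor toward the player.
; When that timeline finishes, it sends IncreaseCollectableValue to the game mode and destroys itself.
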(event OnComponentBeginOverlap(Sphere)
  (params (OverlappedComponent :type Primitive%20Component%20Object%20Reference) (OtherActor :type Actor%20Object%20Reference) (OtherComp :type Primitive%20Component%20Object%20Reference) (OtherBodyIndex :type Integer) (bFromSweep :type Boolean) (SweepResult :type Hit%20Result%20Structure%20%28by%20ref%29))
  (if (== (Utilities|GetClass OtherActor) "/Game/Blueprints/Core/BP_Player.BP_Player_C")
    (Variables|Default|SetHitActor OtherActor)
    (Utilities|FlowControl|DoOnce false
      (:Completed
        (bind __value (Timeline|Collect Play)
          (:Update
            (bind _hitactor (Variables|Default|GetHitActor)
              (:then
                (Transformation|SetActorLocation (Math|Vector|Lerp(Vector) (Transformation|GetActorLocation) (Transformation|GetActorLocation _hitactor) __value) true false))
              (:else)))
          (:Finished
            (Class|BPIGameMode|IncreaseCollectableValue(Message) (Game|GetGameMode) (Variables|Default|GetValue))
            (Actor|DestroyActor)))))))

(event EventBeginPlay
  (bind _scene (Variables|Default|GetScene))
  (bind (_direction _value _sine) (Timeline|CoinRotate Play)
    (:Update
      (Transformation|SetRelativeRotation _scene (Math|Rotator|Lerp(Rotator) "0, 0, 0" "0.000000,180.000000,0.000000" _value true) true false)
      (Transformation|SetRelativeLocation _scene (Math|Vector|Lerp(Vector) "0.000000,0.000000,90.000000" "0.000000,0.000000,100.000000" _sine) true false))))

(event Collision|EventActorBeginOverlap
  (params (OtherActor :type Actor%20Object%20Reference)))

(event EventTick
  (params (DeltaSeconds :type Float%20%28single-precision%29)))

(fn ConstructionScript)