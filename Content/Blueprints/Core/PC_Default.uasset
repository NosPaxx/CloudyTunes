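; Default player controller that sets up input and camera limits and opens the pause and cheat menus.
; On BeginPlay it adds the default Enhanced Input mapping context and clamps the camera's view pitch.
; The pause and cheat actions each push their widget onto the main UI stack, switch to UI-only input, show a centered cursor and pause the game.
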(event Input|EnhancedActionEvents|EnhancedInputActionIA_Pause
  (params (ActionValue :type Boolean) (ElapsedSeconds :type Float%20%28double-precision%29) (TriggeredSeconds :type Float%20%28double-precision%29) (InputAction :type Input%20Action%20Object%20Reference :default "/Game/Inputs/IA_Pause.IA_Pause"))
  (bind _returnvalue (Viewport|GetViewportSize))
  (bind (_x _y) (Math|Vector2D|BreakVector2D _returnvalue))
  (:Started
    (bind _returnvalue_2 (Class|CommonActivatableWidgetContainerBase|AddWidget (CallFunction|ReturnMainStack self) "/Game/UI/CommonUISetup/CAW_Pause.CAW_Pause_C"))
    (Input|SetInputModeUIOnly self _returnvalue_2 "DoNotLock" true)
    (Variables|Default|SetbShowMouseCursor true)
    (Class|PlayerController|SetMouseLocation (/ (Math|Float|Truncate _x) 2) (/ (Math|Float|Truncate _y) 2))
    (Game|SetGamePaused true)))

(event Input|EnhancedActionEvents|EnhancedInputActionIA_Cheat
  (params (ActionValue :type Boolean) (ElapsedSeconds :type Float%20%28double-precision%29) (TriggeredSeconds :type Float%20%28double-precision%29) (InputAction :type Input%20Action%20Object%20Reference :default "/Game/Inputs/IA_Cheat.IA_Cheat"))
  (bind _returnvalue (Viewport|GetViewportSize))
  (bind (_x _y) (Math|Vector2D|BreakVector2D _returnvalue))
  (bind _returnvalue_2 (Class|CommonActivatableWidgetContainerBase|AddWidget (CallFunction|ReturnMainStack self) "/Game/UI/CAW_CheatMenu.CAW_CheatMenu_C"))
  (Input|SetInputModeUIOnly self _returnvalue_2 "DoNotLock" true)
  (Variables|Default|SetbShowMouseCursor true)
  (Class|PlayerController|SetMouseLocation (/ (Math|Float|Truncate _x) 2) (/ (Math|Float|Truncate _y) 2))
  (Game|SetGamePaused true))

(event EventBeginPlay
  (Input|AddMappingContext (PlayerController|LocalPlayerSubsystems|GetEnhancedInputLocalPlayerSubsystem) "/Game/Inputs/IMC_Default.IMC_Default" 0 "(bIgnoreAllPressedKeysUntilRelease=True,bForceImmediately=False,bNotifyUserSettings=False)")
  (Variables|/Script/Engine.PlayerCameraManager|SetViewPitchMax (Game|GetPlayerCameraManager 0) 5e+01)
  (Variables|/Script/Engine.PlayerCameraManager|SetViewPitchMin (Game|GetPlayerCameraManager 0) -8e+01))

(fn ConstructionScript)